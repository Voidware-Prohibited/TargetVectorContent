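; Player character Blueprint that disguises itself as props in the level by copying the static mesh it targets.
; Pressing E fires a short forward sphere trace from the actor on the Visibility channel, with debug drawing on.
; On hitting a plain StaticMeshActor, it copies that mesh, rotation and scale onto its StaticMesh component, setting height from the target's Z minus a fixed offset.
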(event Collision|EventActorBeginOverlap
  (params (OtherActor :type Actor%20Object%20Reference)))

(event EventTick
  (params (DeltaSeconds :type Float%20%28single-precision%29)))

(event Input|KeyboardEvents|E
  (params (Key :type Key%20Structure))
  (bind _returnvalue (Transformation|GetActorLocation))
  (bind _staticmesh (Variables|Default|GetStaticMesh))
  (bind _relativelocation (Variables|/Script/Engine.SceneComponent|GetRelativeLocation _staticmesh))
  (:Pressed
    (bind _outhit (Collision|SphereTraceByChannel _returnvalue (+ _returnvalue (* (Transformation|GetActorForwardVector) 5e+02)) 1e+01 "TraceTypeQuery1" false 0 "ForDuration"))
    (if (.bBlockingHit (Collision|BreakHitResult _outhit))
      (if (== (Utilities|GetClass (.HitActor (Collision|BreakHitResult _outhit))) "/Script/Engine.StaticMeshActor")
        (bind _asstatic_mesh_actor (Utilities|Casting|CastToStaticMeshActor (.HitActor (Collision|BreakHitResult _outhit)))
          (:then
            (Components|StaticMesh|SetStaticMesh (Variables|Default|GetStaticMesh) (Variables|/Script/Engine.StaticMeshComponent|GetStaticMesh (Variables|/Script/Engine.StaticMeshActor|GetStaticMeshComponent _asstatic_mesh_actor)))
            (Transformation|SetRelativeTransform (Variables|Default|GetStaticMesh) (Math|Transform|MakeTransform (Math|Vector|MakeVector (.x _relativelocation) (.y _relativelocation) (- (.z (Variables|/Script/Engine.SceneComponent|GetRelativeLocation (Variables|/Script/Engine.StaticMeshActor|GetStaticMeshComponent _asstatic_mesh_actor))) 104.0)) (Variables|/Script/Engine.SceneComponent|GetRelativeRotation (Variables|/Script/Engine.StaticMeshActor|GetStaticMeshComponent _asstatic_mesh_actor)) (Variables|/Script/Engine.SceneComponent|GetRelativeScale3D (Variables|/Script/Engine.StaticMeshActor|GetStaticMeshComponent _asstatic_mesh_actor))) false true))
          (:CastFailed
            (Development|PrintString "Hello")))))))

(fn ConstructionScript)