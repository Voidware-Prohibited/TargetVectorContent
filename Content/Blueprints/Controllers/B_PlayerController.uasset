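; Player controller for an ALSXT-based game that sets the game instance state and handles local input setup, menus and debug controls.
; On BeginPlay, the local controller swaps in ALSXT Enhanced Input mapping contexts and adds a GameplayTasks component.
; Input events reach the HUD through message calls to open the in-game menu, toggle the EOS menu and drive the overlay-mode selector.
; Debug inputs toggle UI, ALS ShowDebug views and slow motion, with time dilation limited to standalone.
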(event Input|EnhancedActionEvents|EnhancedInputActionIA_Back
  (params (ActionValue :type Boolean) (ElapsedSeconds :type Float%20%28double-precision%29) (TriggeredSeconds :type Float%20%28double-precision%29) (InputAction :type Input%20Action%20Object%20Reference :default "/ALSXT/ALS/Data/Input/IA_Back.IA_Back"))
  (:Triggered
    (bind _active (Class|BIHUD|IsinGameMainMenuActive(Message) (HUD|GetHUD)))
    (if (not _active)
      (Class|BIHUD|DisplayinGameMainMenu(Message) (HUD|GetHUD)))))

(event EventBeginPlay
  (Class|BIGameInstance|SetInstanceState(Message) (Game|GetGameInstance) "NewEnumerator2")
  (|InitializeLocalPlayer))

(fn ConstructionScript)

(fn SetGlobalTimeDilation
  (params (Time%20Dilation :type Float%20%28double-precision%29))
  (if (Class|KismetSystemLibrary|IsStandalone)
    (Utilities|Time|SetGlobalTimeDilation Time%20Dilation)))

(event Input|EnhancedActionEvents|EnhancedInputActionIA_OverlayModeMenu
  (params (ActionValue :type Boolean) (ElapsedSeconds :type Float%20%28double-precision%29) (TriggeredSeconds :type Float%20%28double-precision%29) (InputAction :type Input%20Action%20Object%20Reference :default "/ALS/ALSExtras/Data/Input/IA_OverlayModeMenu.IA_OverlayModeMenu"))
  (:Triggered
    (bind _overlay_menu (Class|BIHUD|GetOverlayMenu(Message) (HUD|GetHUD)))
    (if ActionValue
      (if (Variables|State|GetbSlomoActive)
        _
        (else
          (CallFunction|SetGlobalTimeDilation 0.35)))
      (UserInterface|Viewport|AddtoViewport _overlay_menu 0)
      (else
        (if (Variables|State|GetbSlomoActive)
          _
          (else
            (CallFunction|SetGlobalTimeDilation 1.0)))
        (Default|ApproveOverlayMode _overlay_menu)
        (Widget|RemovefromParent _overlay_menu)))))

(event Input|EnhancedActionEvents|EnhancedInputActionIA_NextOverlayMode
  (params (ActionValue :type Boolean) (ElapsedSeconds :type Float%20%28double-precision%29) (TriggeredSeconds :type Float%20%28double-precision%29) (InputAction :type Input%20Action%20Object%20Reference :default "/ALS/ALSExtras/Data/Input/IA_NextOverlayMode.IA_NextOverlayMode"))
  (:Triggered
    (bind _overlay_menu (Class|BIHUD|GetOverlayMenu(Message) (HUD|GetHUD)))
    (if (UserInterface|Viewport|IsinViewport _overlay_menu)
      (Default|CycleOverlayMode _overlay_menu true))))

(event Input|EnhancedActionEvents|EnhancedInputActionIA_PreviousOverlayMode
  (params (ActionValue :type Boolean) (ElapsedSeconds :type Float%20%28double-precision%29) (TriggeredSeconds :type Float%20%28double-precision%29) (InputAction :type Input%20Action%20Object%20Reference :default "/ALS/ALSExtras/Data/Input/IA_PreviousOverlayMode.IA_PreviousOverlayMode"))
  (:Triggered
    (bind _overlay_menu (Class|BIHUD|GetOverlayMenu(Message) (HUD|GetHUD)))
    (if (UserInterface|Viewport|IsinViewport _overlay_menu)
      (Default|CycleOverlayMode _overlay_menu false))))

(event Input|EnhancedActionEvents|EnhancedInputActionIA_ToggleUI
  (params (ActionValue :type Boolean) (ElapsedSeconds :type Float%20%28double-precision%29) (TriggeredSeconds :type Float%20%28double-precision%29) (InputAction :type Input%20Action%20Object%20Reference :default "/ALS/ALSExtras/Data/Input/IA_ToggleUI.IA_ToggleUI"))
  (:Triggered
    (Variables|State|SetbUIVisible (not (Variables|State|GetbUIVisible)))))

(event Input|EnhancedActionEvents|EnhancedInputActionIA_Slomo
  (params (ActionValue :type Boolean) (ElapsedSeconds :type Float%20%28double-precision%29) (TriggeredSeconds :type Float%20%28double-precision%29) (InputAction :type Input%20Action%20Object%20Reference :default "/ALS/ALSExtras/Data/Input/IA_Slomo.IA_Slomo"))
  (:Triggered
    (Variables|State|SetbSlomoActive (not (Variables|State|GetbSlomoActive)))
    (CallFunction|SetGlobalTimeDilation (Math|Float|SelectFloat 0.15 1.0 (Variables|State|GetbSlomoActive)))))

(event Input|ActionEvents|InputActionOpenMenu
  (params (Key :type Key%20Structure))
  (bind _self self)
  (bind _self_2 self)
  (:Pressed
    (if (Pawn|IsLocalPlayerController)
      (Variables|Default|GetEOSMenu
        (:then
          (bind _game_layer_stack (Class|BIHUD|GetGameLayerStack(Message) (HUD|GetHUD)))
          (Class|CommonActivatableWidgetContainerBase|RemoveWidget _game_layer_stack (Variables|Default|GetEOSMenu))
          (Variables|Default|SetEOSMenu 0)
          (Variables|/Script/Engine.PlayerController|SetbShowMouseCursor _self_2 false)
          (Input|SetInputModeGameOnly _self_2))
        (:else
          (bind _game_layer_stack_2 (Class|BIHUD|GetGameLayerStack(Message) (HUD|GetHUD)))
          (bind _returnvalue (Class|CommonActivatableWidgetContainerBase|AddWidget _game_layer_stack_2 "/TargetVectorCommonUI/Widgets/Utility/Common_EOS.Common_EOS_C"))
          (bind _output_get (Variables|Default|SetEOSMenu _returnvalue))
          (Input|SetInputModeGameandUI _self _output_get "LockAlways" true)
          (Variables|/Script/Engine.PlayerController|SetbShowMouseCursor _self true))))))

(event Input|KeyboardEvents|DebugKeyShift1
  (params (Key :type Key%20Structure) (ActionValue :type Input%20Action%20Value%20Structure))
  (:Pressed
    (Development|ExecuteConsoleCommand "ShowDebug ALS.Curves" self)))

(event Input|KeyboardEvents|DebugKeyShift0
  (params (Key :type Key%20Structure) (ActionValue :type Input%20Action%20Value%20Structure))
  (:Pressed
    (Development|ExecuteConsoleCommand "ShowDebug" self)))

(event Input|KeyboardEvents|DebugKeyShift2
  (params (Key :type Key%20Structure) (ActionValue :type Input%20Action%20Value%20Structure))
  (:Pressed
    (Development|ExecuteConsoleCommand "ShowDebug ALS.State" self)))

(event Input|KeyboardEvents|DebugKeyShift3
  (params (Key :type Key%20Structure) (ActionValue :type Input%20Action%20Value%20Structure))
  (:Pressed
    (Development|ExecuteConsoleCommand "ShowDebug ALS.Shapes" self)))

(event Input|KeyboardEvents|DebugKeyShift4
  (params (Key :type Key%20Structure) (ActionValue :type Input%20Action%20Value%20Structure))
  (:Pressed
    (Development|ExecuteConsoleCommand "ShowDebug ALS.Traces" self)))

(event Input|KeyboardEvents|DebugKeyShift5
  (params (Key :type Key%20Structure) (ActionValue :type Input%20Action%20Value%20Structure))
  (:Pressed
    (Development|ExecuteConsoleCommand "ShowDebug ALS.Mantling" self)))

(event Input|KeyboardEvents|DebugKeyShift6
  (params (Key :type Key%20Structure) (ActionValue :type Input%20Action%20Value%20Structure))
  (:Pressed
    (Development|ExecuteConsoleCommand "ShowDebug ALS.CameraCurves" self)))

(event Input|KeyboardEvents|DebugKeyShift7
  (params (Key :type Key%20Structure) (ActionValue :type Input%20Action%20Value%20Structure))
  (:Pressed
    (Development|ExecuteConsoleCommand "ShowDebug ALS.CameraShapes" self)))

(event Input|KeyboardEvents|DebugKeyShift8
  (params (Key :type Key%20Structure) (ActionValue :type Input%20Action%20Value%20Structure))
  (:Pressed
    (Development|ExecuteConsoleCommand "ShowDebug ALS.CameraTraces" self)))